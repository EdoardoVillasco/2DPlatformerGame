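; Enemy AI controller that runs BT_Enemy on possess and starts it in a Passive state.
; Perception updates check each actor for sight and damage stimuli via a helper that matches sense classes.
; While Passive, seeing the player or sensing damage from any actor switches to Attacking.
; State and attack target are written to the Blackboard, and nothing here returns the enemy to Passive after attacking.
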(event OnPerceptionUpdated(AIPerception)
  (params (UpdatedActors :type Array%20of%20Actor%20Object%20References))
  (for _array_element UpdatedActors
    (Utilities|FlowControl|Sequence
      (:then_0
        (bind _sensed (CallFunction|CanSenseActor _array_element "NewEnumerator1"))
        (if _sensed
          (CallFunction|HandleSensedSight _array_element)))
      (:then_1
        (bind _sensed_2 (CallFunction|CanSenseActor _array_element "NewEnumerator2"))
        (if _sensed_2
          (CallFunction|HandleSensedDamage _array_element))))))

(event EventPossess
  (params (PossessedPawn :type Pawn%20Object%20Reference))
  (AI|RunBehaviorTree "/Game/Blueprints/AI/BT_Enemy.BT_Enemy")
  (CallFunction|SetStateasPassive))

(fn ConstructionScript)

(fn SetStateasPassive
  (AI|Components|Blackboard|SetValueasEnum (Variables|Default|GetBlackboard) (Variables|Default|GetStateKeyName) (Utilities|Enum|LiteralenumE_AIState "NewEnumerator0")))

(fn SetStateasAttacking
  (params (AttackTarget :type Actor%20Object%20Reference))
  (AI|Components|Blackboard|SetValueasObject (Variables|Default|GetBlackboard) (Variables|Default|GetAttackTargetKeyName) AttackTarget)
  (AI|Components|Blackboard|SetValueasEnum (Variables|Default|GetBlackboard) (Variables|Default|GetStateKeyName) (Utilities|Enum|LiteralenumE_AIState "NewEnumerator1")))

(fn CanSenseActor
  (params (Actor :type Actor%20Object%20Reference) (Snese :type E_AISense%20Enum :default "NewEnumerator0"))
  (bind _info (Class|AIPerceptionComponent|GetActorsPerception (Variables|Default|GetAIPerception) Actor))
  (for _array_element (.LastSensedStimuli (Utilities|Struct|BreakActorPerceptionBlueprintInfo _info))
    (bind _returnvalue (Class|AIPerceptionSystem|GetSenseClassforStimulus _array_element))
    (if (== _returnvalue (Utilities|Select :Index Snese :NewEnumerator0 0 :NewEnumerator1 "/Script/AIModule.AISense_Sight" :NewEnumerator2 "/Script/AIModule.AISense_Damage"))
      (return (.bSuccessfullySensed (Utilities|Struct|BreakAIStimulus _array_element)) _array_element))))

(fn HandleSensedSight
  (params (Actor :type Actor%20Object%20Reference))
  (bind _state (CallFunction|GetCurrentState))
  (switch Utilities|FlowControl|Switch|SwitchonE_AIState _state
    (:NewEnumerator0
      (if (== Actor (Game|GetPlayerCharacter 0))
        (CallFunction|SetStateasAttacking Actor)))))

(fn GetCurrentState
  (return (Utilities|Enum|ByteToEnumE_AIState (Class|BlackboardComponent|GetValueasEnum (Variables|Default|GetBlackboard) (Variables|Default|GetStateKeyName)))))

(fn HandleSensedDamage
  (params (Actor :type Actor%20Object%20Reference))
  (bind _state (CallFunction|GetCurrentState))
  (switch Utilities|FlowControl|Switch|SwitchonE_AIState _state
    (:NewEnumerator0
      (CallFunction|SetStateasAttacking Actor))))