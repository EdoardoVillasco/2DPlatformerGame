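; BP_PatrolRoute is a spline-based patrol path for AI that tracks a current point index along its PatrolRoute spline.
; IncrementPatrolRoute steps the index by Direction and flips that direction at the first and last points, producing a back-and-forth route rather than a loop.
; GetSplinePointAsWorldPosition returns the world location of the current point.
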(event Custom|IncrementPatrolRoute
  (bind _output_get (Variables|PatrolRoute|SetPatrolIndex (+ (Variables|PatrolRoute|GetPatrolIndex) (Variables|PatrolRoute|GetDirection))))
  (if (== _output_get (- (Spline|GetNumberOfSplinePoints (Variables|Default|GetPatrolRoute)) 1))
    (Variables|PatrolRoute|SetDirection -1)
    (elif (== (Variables|PatrolRoute|GetPatrolIndex) 0)
      (Variables|PatrolRoute|SetDirection 1))))

(fn ConstructionScript)

(fn GetSplinePointasWorldPosition
  (return (Spline|GetLocationatSplinePoint (Variables|Default|GetPatrolRoute) (Variables|PatrolRoute|GetPatrolIndex) "World")))