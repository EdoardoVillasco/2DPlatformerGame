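; BP_Shop is a shop actor that opens an upgrade menu when the player interacts within its trigger.
; Entering the ShopTrigger enables input on the actor and shows WBP_Interact; leaving disables input and removes the prompt.
; Interact switches the view to the shop, opens WBP_Upgrade with UI-only input and cursor, hides the player and blocks movement.
; Nothing here restores that state, and a WBP_ShopKeeper creation node is left unconnected.
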(event OnComponentBeginOverlap(ShopTrigger)
  (params (OverlappedComponent :type Primitive%20Component%20Object%20Reference) (OtherActor :type Actor%20Object%20Reference) (OtherComp :type Primitive%20Component%20Object%20Reference) (OtherBodyIndex :type Integer) (bFromSweep :type Boolean) (SweepResult :type Hit%20Result%20Structure%20%28by%20ref%29))
  (if (== OtherActor (Game|Player|GetPlayerPawn 0))
    (Input|EnableInput (Game|GetPlayerController 0))
    (bind _returnvalue (UserInterface|CreateWidget "/Game/Blueprints/Widgets/WBP_Interact.WBP_Interact_C"))
    (UserInterface|Viewport|AddtoViewport _returnvalue 0)))

(event OnComponentEndOverlap(ShopTrigger)
  (params (OverlappedComponent :type Primitive%20Component%20Object%20Reference) (OtherActor :type Actor%20Object%20Reference) (OtherComp :type Primitive%20Component%20Object%20Reference) (OtherBodyIndex :type Integer))
  (if (== OtherActor (Game|Player|GetPlayerPawn 0))
    (Input|DisableInput (Game|GetPlayerController 0))
    (bind _foundwidgets (Widget|GetAllWidgetsOfClass "/Game/Blueprints/Widgets/WBP_Interact.WBP_Interact_C" true))
    (Widget|RemovefromParent _foundwidgets)))

(event EventInteract
  (bind _returnvalue (Game|GetPlayerController 0))
  (Game|Player|SetViewTargetwithBlend (Game|GetPlayerController 0) self 0.0 "VTBlend_Linear" 0.0 false)
  (bind _returnvalue_2 (UserInterface|CreateWidget "/Game/Blueprints/Widgets/WBP_Upgrade.WBP_Upgrade_C"))
  (UserInterface|Viewport|AddtoViewport _returnvalue_2 0)
  (Input|SetInputModeUIOnly _returnvalue _returnvalue_2 "DoNotLock" false)
  (Variables|/Script/Engine.PlayerController|SetbShowMouseCursor _returnvalue true)
  (Rendering|SetActorHiddenInGame (Game|GetPlayerCharacter 0) true)
  (Input|SetIgnoreMoveInput (Game|GetPlayerController 0) true))

(fn ConstructionScript)